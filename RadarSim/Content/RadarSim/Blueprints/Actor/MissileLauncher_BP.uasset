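; Missile launcher actor for the radar sim that manages the missiles mounted on it.
; On BeginPlay it runs parent logic, then passes its missile array to a routine that gathers missiles attached from the start.
; SpawnMissile creates the configured missile type at the launcher's transform, records it and attaches it to the launcher mesh.
; EditorRemoveMissile pops the last array entry and destroys that actor if valid.
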(event Custom|SpawnMissile
  (bind _returnvalue (Transformation|GetActorTransform))
  (bind _returnvalue_2 (Game|SpawnActorfromClass (Class|MissileLauncher|GetMissileType) (Math|Transform|MakeTransform (.location _returnvalue) (.rotation _returnvalue) "1.000000,1.000000,1.000000") "Undefined" "MultiplyWithRoot" 0 0))
  (Utilities|Array|Add (Variables|Missile|GetMissile_BP_Init) _returnvalue_2)
  (Transformation|AttachComponentToComponent _returnvalue_2 (Variables|Default|GetmissileLauncherMesh) "None" "KeepWorld" "KeepWorld" "KeepWorld" true))

(event Custom|Editor%20Remove%20Missile
  (CallFunction|RemoveMissile))

(event EventBeginPlay
  (|CallParentFunction)
  (Class|MissileLauncher|GetMissileAttachedtoMissileLauncherfromStart (Variables|Missile|GetMissile_BP_Init)))

(event Collision|EventActorBeginOverlap
  (params (OtherActor :type Actor%20Object%20Reference)))

(event EventTick
  (params (DeltaSeconds :type Float%20%28single-precision%29)))

(fn ConstructionScript)

(fn RemoveMissile
  (bind _missile_bp_init (Variables|Missile|GetMissile_BP_Init))
  (bind _returnvalue (Utilities|Array|Length _missile_bp_init))
  (bind _returnvalue_2 (- _returnvalue 1))
  (if (< _returnvalue_2 _returnvalue)
    (bind _output_get (LocalVariables|SetActorToDestroy (Utilities|Array|Get(acopy) _missile_bp_init _returnvalue_2)))
    (Utilities|Array|RemoveIndex _missile_bp_init _returnvalue_2)
    (Utilities|IsValid _output_get
      (:Is%20Valid
        (Actor|DestroyActor _output_get)))))